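; Game Instance Blueprint for a TicTacToe game that applies display and performance settings at startup.
; The Init event runs a fixed chain of console commands to set a small square windowed resolution.
; The same chain caps frame rate, disables vsync and lowers shadow, texture, effects, post-process, detail and view distance settings for a lightweight render load.
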(event `self.ReceiveInit`
  (`KismetSystemLibrary.ExecuteConsoleCommand` "r.SetRes 640x640w" null) ; windowed 640x640
  (`KismetSystemLibrary.ExecuteConsoleCommand` "sg.ShadowQuality 0" null)
  (`KismetSystemLibrary.ExecuteConsoleCommand` "t.maxfps 30" null)
  (`KismetSystemLibrary.ExecuteConsoleCommand` "r.ScreenPercentage 100" null)
  (`KismetSystemLibrary.ExecuteConsoleCommand` "r.ViewDistanceScale 0.4" null)
  (`KismetSystemLibrary.ExecuteConsoleCommand` "r.SkeletalMeshLODBias 1" null)
  (`KismetSystemLibrary.ExecuteConsoleCommand` "r.PostProcessAAQuality 0" null)
  (`KismetSystemLibrary.ExecuteConsoleCommand` "sg.PostProcessQuality 0" null)
  (`KismetSystemLibrary.ExecuteConsoleCommand` "sg.TextureQuality 0" null)
  (`KismetSystemLibrary.ExecuteConsoleCommand` "sg.EffectsQuality 0" null)
  (`KismetSystemLibrary.ExecuteConsoleCommand` "r.DetailMode 0" null)
  (`KismetSystemLibrary.ExecuteConsoleCommand` "FoliageQuality 0" null)
  (`KismetSystemLibrary.ExecuteConsoleCommand` "r.vsync 0" null))